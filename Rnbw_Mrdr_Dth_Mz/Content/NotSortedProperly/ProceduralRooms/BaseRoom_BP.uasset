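; BaseRoom_BP is a room Blueprint for procedural rooms that randomises its floor look and occasional powerup.
; Its construction script has a 1-in-21 chance to call SpawnPowerup, which adds a child actor component at the ItemSpawn transform.
; It also gives each GroundTiles child mesh one of two dynamic materials at random, tinting only the Base_02 tiles with a random colour.
; SetAttachPoints is an empty stub.
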(event EventBeginPlay)

(event Collision|EventActorBeginOverlap
  (params (OtherActor :type Actor%20Object%20Reference)))

(event EventTick
  (params (DeltaSeconds :type Float%20%28single-precision%29)))

(fn ConstructionScript
  (bind _max (LocalVariables|Getmax))
  (bind _min (LocalVariables|GetMin))
  (if (== (Math|Random|RandomIntegerinRange 0 20) 10)
    (CallFunction|SpawnPowerup))
  ;[1 1 1] Floor tile colours
  (for _array_element (Components|GetChildrenComponents (Variables|Default|GetGroundTiles) false)
    (bind _asstatic_mesh_component (Utilities|Casting|CastToStaticMeshComponent _array_element))
    (if (Math|Random|RandomBool)
      (Rendering|Material|CreateDynamicMaterialInstance _asstatic_mesh_component 0 "/Game/NotSortedProperly/MultistoryDungeons/Materials/Base_01.Base_01" "None" :!class /Script/Engine.PrimitiveComponent)
      (else
        (bind _returnvalue (Rendering|Material|CreateDynamicMaterialInstance _asstatic_mesh_component 0 "/Game/NotSortedProperly/MultistoryDungeons/Materials/Base_02.Base_02" "None" :!class /Script/Engine.PrimitiveComponent))
        (Rendering|Material|SetVectorParameterValue _returnvalue "Base Colour" (Math|Color|MakeColor (Math|Random|RandomFloatinRange _min _max) (Math|Random|RandomFloatinRange _min _max) (Math|Random|RandomFloatinRange _min _max)) :!class /Script/Engine.MaterialInstanceDynamic)))))

(fn SetAttachPoints)

(fn SpawnPowerup
  (AddComponent|AddChildActorComponent false (Transformation|GetRelativeTransform (Variables|Default|GetItemSpawn))))