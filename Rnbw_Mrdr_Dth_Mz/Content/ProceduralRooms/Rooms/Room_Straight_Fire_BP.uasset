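; Straight procedural room Blueprint with a fire hazard that damages the adventurer character.
; Entering the Capsule trigger deals damage immediately and sets a Burned flag, which any end overlap on the capsule clears.
; A Delay on Tick acts as a repeating timer, damaging the stored character about every 1.75 seconds while the flag is set.
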(event OnComponentBeginOverlap(Capsule)
  (params (OverlappedComponent :type Primitive%20Component%20Object%20Reference) (OtherActor :type Actor%20Object%20Reference) (OtherComp :type Primitive%20Component%20Object%20Reference) (OtherBodyIndex :type Integer) (bFromSweep :type Boolean) (SweepResult :type Hit%20Result%20Structure%20%28by%20ref%29))
  (bind _asadventurer_character (Utilities|Casting|CastToAdventurerCharacter OtherActor))
  (Default|TakeDamage _asadventurer_character)
  (Variables|Default|SetBurned? true))

(event OnComponentEndOverlap(Capsule)
  (params (OverlappedComponent :type Primitive%20Component%20Object%20Reference) (OtherActor :type Actor%20Object%20Reference) (OtherComp :type Primitive%20Component%20Object%20Reference) (OtherBodyIndex :type Integer))
  (Variables|Default|SetBurned? false))

(event EventBeginPlay
  (|CallParentFunction) ; This node is disabled and will not be called.\nDrag off pins to build functionality.
)

(event Collision|EventActorBeginOverlap
  (params (OtherActor :type Actor%20Object%20Reference))
  (|CallParentFunction OtherActor) ; This node is disabled and will not be called.\nDrag off pins to build functionality.
)

(event EventTick
  (params (DeltaSeconds :type Float%20%28single-precision%29))
  (Utilities|FlowControl|Delay 1.75)
  (if (Variables|Default|GetBurned?)
    (Default|TakeDamage (stale OnComponentBeginOverlap(Capsule) _asadventurer_character))))

(fn ConstructionScript
  (|CallParentFunction))